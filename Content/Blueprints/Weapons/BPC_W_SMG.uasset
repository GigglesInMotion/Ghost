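; SMG weapon Blueprint, built on a parent class, that sets up the SMG11 weapon's skeletal mesh.
; The construction script runs the parent's script, then uses the NewOld boolean to pick the SMG11_X or SMG11_Nostock_X mesh for WeaponMesh, reinitializing the pose.
; The event graph holds only disabled placeholder events, so this Blueprint adds no runtime logic of its own.
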(event EventBeginPlay
  (|CallParentFunction) ; This node is disabled and will not be called.\nDrag off pins to build functionality.
)

(event Collision|EventActorBeginOverlap
  (params (OtherActor :type Actor%20Object%20Reference))
  (|CallParentFunction OtherActor) ; This node is disabled and will not be called.\nDrag off pins to build functionality.
)

(event EventTick
  (params (DeltaSeconds :type Float%20%28single-precision%29))
  (|CallParentFunction DeltaSeconds) ; This node is disabled and will not be called.\nDrag off pins to build functionality.
)

(fn ConstructionScript
  (|CallParentFunction)
  (Class|SkinnedMeshComponent|SetSkeletalMesh (Variables|Default|GetWeaponMesh) (select (Variables|Default|GetNew/Old) "/Game/ExternalContent/FPS_Test_Weapons/Weapons/Meshes/SMG11/SK_SMG11_X.SK_SMG11_X" "/Game/ExternalContent/FPS_Test_Weapons/Weapons/Meshes/SMG11/SK_SMG11_Nostock_X.SK_SMG11_Nostock_X") true))