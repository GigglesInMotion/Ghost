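; Weapon Blueprint that acts as a world object the player can detect when nearby and that carries its own weapon data.
; Collision overlap with BP_Player caches the player, sets PlayerInRange and registers itself as the player's WeaponInRange.
; End overlap only clears PlayerInRange, for any actor, leaving the player's reference set.
; The construction script rebuilds the Weapon struct, keeping most fields while filling in its class, a fixed enum value and WeaponMesh.
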(event OnComponentBeginOverlap(Collision)
  (params (OverlappedComponent :type Primitive%20Component%20Object%20Reference) (OtherActor :type Actor%20Object%20Reference) (OtherComp :type Primitive%20Component%20Object%20Reference) (OtherBodyIndex :type Integer) (bFromSweep :type Boolean) (SweepResult :type Hit%20Result%20Structure%20%28by%20ref%29))
  (bind _asbp_player (Utilities|Casting|CastToBP_Player OtherActor))
  (bind _output_get (Variables|Default|SetPlayer _asbp_player))
  (Variables|Default|SetPlayerInRange? true)
  (Variables|/Game/Blueprints/Player/BP_Player.BP_Player_C|SetWeaponInRange _output_get self))

(event OnComponentEndOverlap(Collision)
  (params (OverlappedComponent :type Primitive%20Component%20Object%20Reference) (OtherActor :type Actor%20Object%20Reference) (OtherComp :type Primitive%20Component%20Object%20Reference) (OtherBodyIndex :type Integer))
  (Variables|Default|SetPlayerInRange? false))

(fn ConstructionScript
  (Variables|Default|SetWeapon (Utilities|Struct|MakeStr_Weapon (.type (Variables|Default|GetWeapon)) (Utilities|GetClass self) (.name (Variables|Default|GetWeapon)) (.equipsocket (Variables|Default|GetWeapon)) (.unequipsocket (Variables|Default|GetWeapon)) (.damage (Variables|Default|GetWeapon)) (.range (Variables|Default|GetWeapon)) (.firerate (Variables|Default|GetWeapon)) (.magazinesize (Variables|Default|GetWeapon)) (.currentammo (Variables|Default|GetWeapon)) "NewEnumerator0" (Variables|Default|GetWeaponMesh))))